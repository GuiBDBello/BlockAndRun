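; Turret actor that fires projectiles at a ThirdPersonCharacter while the character is within its sphere trigger.
; Sphere overlap begin and end set or clear the target and the shoot flag.
; Tick runs through a one-second Delay, throttling fire to roughly one TurretProjectile per second.
; Each projectile spawns at the turret's location, rotated toward the target, and receives that target as a parameter.
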(event `self.ReceiveTick`
  (params (DeltaSeconds :type "Float (single-precision)"))
  (bind _returnvalue (`self.K2_GetActorLocation`))
  (bind _target (`self.Target`))
  (`KismetSystemLibrary.Delay` 1.0)
  (if (`self.Shoot`)
    (`|SpawnActorFromClass` "/Game/Bounds/TurretProjectile.TurretProjectile_C" (`KismetMathLibrary.MakeTransform` _returnvalue (`KismetMathLibrary.FindLookAtRotation` _returnvalue (`self.K2_GetActorLocation` _target))) "Undefined" "OverrideRootScale" null _target null)))

(event `self.Sphere.OnComponentBeginOverlap`
  (params (OverlappedComponent :type "PrimitiveComponent Object Reference") (OtherActor :type "Actor Object Reference") (OtherComp :type "PrimitiveComponent Object Reference") (OtherBodyIndex :type Integer) (bFromSweep :type Boolean) (SweepResult :type "HitResult Structure (by ref)"))
  (bind _asthird_person_character (cast `/Game/ThirdPersonBP/Blueprints/ThirdPersonCharacter` OtherActor))
  (set `self.Target` _asthird_person_character)
  (set `self.Shoot` true))

(event `self.Sphere.OnComponentEndOverlap`
  (params (OverlappedComponent :type "PrimitiveComponent Object Reference") (OtherActor :type "Actor Object Reference") (OtherComp :type "PrimitiveComponent Object Reference") (OtherBodyIndex :type Integer))
  (cast `/Game/ThirdPersonBP/Blueprints/ThirdPersonCharacter` OtherActor)
  (set `self.Target` null)
  (set `self.Shoot` false))

(fn `UserConstructionScript`)